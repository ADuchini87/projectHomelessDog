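; Enemy character with a PawnSensing component, whose AI is driven by the EnemyBT behavior tree.
; BeginPlay gets its AI controller and starts that tree.
; The OnSeePawn event is empty.
; Disconnected leftover nodes hold an unused sight-pursuit prototype that toggles SeePawn, sets walk speed, moves to the ThirdPersonCharacter and prints debug messages.
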(event `self.ReceiveBeginPlay`
  (`AIController.RunBehaviorTree` (`AIBlueprintHelperLibrary.GetAIController` self) "/Game/_HomelessDog/Blueprints/ADuchini_BP/EnemyBT.EnemyBT"))

(event `self.PawnSensing.OnSeePawn`
  (params (Pawn :type "Pawn Object Reference")))

(fn `UserConstructionScript`)
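; AI controller for AI_Character pawns, likely dogs, that reacts to spotting the WOLF character and runs the AI_BT behavior tree on possession.
; Perception updates on the WOLF write the SeePlayer blackboard flag.
; When sight is gained it also stores the pawn's location as LastLocationBeforeChase, sets AfterChase and plays a bark at the pawn.
; When sight is lost it plays a growl instead.
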(event `self.OnPossess`
  (params (PossessedPawn :type "Pawn Object Reference"))
  (cast `/Game/_HomelessDog/Blueprints/Enemy/AI_Character` PossessedPawn)
  (`self.RunBehaviorTree` "/Game/_HomelessDog/Blueprints/AI/AI_BT.AI_BT"))

(event `self.AIPerception.OnTargetPerceptionUpdated`
  (params (Actor :type "Actor Object Reference") (Stimulus :type "AIStimulus Structure"))
  (bind (_age _expirationage _strength _stimuluslocation _receiverlocation _tag _bsuccessfullysensed) (break `AIStimulus` Stimulus))
  (bind _returnvalue (`AIBlueprintHelperLibrary.GetBlackboard` null))
  (bind _returnvalue_2 (`self.K2_GetActorLocation` (`self.K2_GetPawn`)))
  (cast `/Game/_HomelessDog/Blueprints/WOLF` Actor)
  (`BlackboardComponent.SetValueAsBool` (`AIBlueprintHelperLibrary.GetBlackboard` null) "SeePlayer" _bsuccessfullysensed)
  (if _bsuccessfullysensed
    (`BlackboardComponent.SetValueAsVector` _returnvalue "LastLocationBeforeChase" _returnvalue_2)
    (`BlackboardComponent.SetValueAsBool` _returnvalue "AfterChase" true)
    (`GameplayStatics.PlaySoundAtLocation` "/Game/_HomelessDog/Blueprints/Sounds/AI_DogBark_Cue.AI_DogBark_Cue" _returnvalue_2 (struct) 1.0 1.0 0.0 null null null)
    (else
      (`GameplayStatics.PlaySoundAtLocation` "/Game/_HomelessDog/Blueprints/Sounds/AI_DogGrowl_Cue.AI_DogGrowl_Cue" _returnvalue_2 (struct) 1.0 1.0 0.0 null null null))))

(fn `UserConstructionScript`)
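; Enemy AI character that chases at speed and bites the WOLF character through a Box overlap.
; Each tick, stamina control reads the SeePlayer blackboard key: it runs and drains stamina while the player is seen, and walks to recover when tired or out of sight.
; Box overlap toggles IsBiting and the wolf's ReceiveDamage flag, dealing damage on contact and repeating through a Tick-driven Delay while biting.
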(event `self.ReceiveTick`
  (params (DeltaSeconds :type "Float (single-precision)"))
  (`self.ControlStamina`)
  (if (`self.IsBiting`)
    (`KismetSystemLibrary.Delay` 0.6)
    (`/Game/_HomelessDog/Blueprints/WOLF.TakeDamage` (stale `self.Box.OnComponentBeginOverlap` _aswolf) (`self.Damage`) :!label _label)))

(event `self.Box.OnComponentBeginOverlap`
  (params (OverlappedComponent :type "PrimitiveComponent Object Reference") (OtherActor :type "Actor Object Reference") (OtherComp :type "PrimitiveComponent Object Reference") (OtherBodyIndex :type Integer) (bFromSweep :type Boolean) (SweepResult :type "HitResult Structure (by ref)"))
  (bind _aswolf (cast `/Game/_HomelessDog/Blueprints/WOLF` OtherActor))
  (bind _output_get (set `self.IsBiting` true))
  (set `/Game/_HomelessDog/Blueprints/WOLF.ReceiveDamage` _output_get _aswolf)
  (goto _label))

(event `self.Box.OnComponentEndOverlap`
  (params (OverlappedComponent :type "PrimitiveComponent Object Reference") (OtherActor :type "Actor Object Reference") (OtherComp :type "PrimitiveComponent Object Reference") (OtherBodyIndex :type Integer))
  (bind _aswolf (cast `/Game/_HomelessDog/Blueprints/WOLF` OtherActor))
  (bind _output_get (set `self.IsBiting` false))
  (set `/Game/_HomelessDog/Blueprints/WOLF.ReceiveDamage` _output_get _aswolf))

(fn `ControlStamina`
  (bind _charactermovement (`self.CharacterMovement`))
  (if (`BlackboardComponent.GetValueAsBool` (`AIBlueprintHelperLibrary.GetBlackboard` (`AIBlueprintHelperLibrary.GetAIController` self)) "SeePlayer")
    (if (`self.IsTired`)
      (set `CharacterMovementComponent.MaxWalkSpeed` 100.0 _charactermovement)
      (`self.IncreaseStamina`)
      (else
        (set `CharacterMovementComponent.MaxWalkSpeed` 350.0 _charactermovement)
        (`self.DecreaseStamina`)))
    (else
      (set `CharacterMovementComponent.MaxWalkSpeed` 100.0 (`self.CharacterMovement`))
      (if (<= (`self.Stamina`) (`self.StaminaMax`))
        (`self.IncreaseStamina`)))))

(fn `DecreaseStamina`
  (bind _output_get (set `self.Stamina` (- (`self.Stamina`) (`self.Stamina2Reduce`))))
  (if (<= _output_get (`self.StaminaMin`))
    (set `self.IsTired` true)))

(fn `GetIsBiting`
  (returns (isBitting :type Boolean))
  (return (`self.IsBiting`)))

(fn `IncreaseStamina`
  (bind _output_get (set `self.Stamina` (+ (`self.Stamina`) (`self.Stamina2Increase`))))
  (if (>= _output_get (`self.StaminaMax`))
    (set `self.IsTired` false)))

(fn `UserConstructionScript`)
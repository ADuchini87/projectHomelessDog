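; Food or drink pickup that raises the wolf's hunger (Hambre) or thirst (Sed) value, then destroys itself.
; The IsComida flag selects which mesh is visible and which stat increases.
; Overlap events detect the player by the display name "WOLF", and Tick consumes the item while overlapping once F registers.
; Both F press and release set IsPressed true, so it never resets and later overlaps consume immediately.
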(event `Key|F` :consume false
  (params (Key :type "Key Structure"))
  ;[1 1 1] ENable input
  (:`Pressed`
    (set `self.is_pressed` true))
  (:`Released`
    (set `self.is_pressed` true)))

(event `self.ReceiveBeginPlay`
  ;[1 1 1] ENable input
  (`self.EnableInput` (`GameplayStatics.GetPlayerController` 0))
  (if (`self.Is_Comida`)
    (`SceneComponent.SetVisibility` (`self.StaticMesh`) false false)
    (`SceneComponent.SetVisibility` (`self.Comida_bebida`) true false)
    (else
      (`SceneComponent.SetVisibility` (`self.StaticMesh`) true false)
      (`SceneComponent.SetVisibility` (`self.Comida_bebida`) false false))))

(event `self.Comida_bebida.OnComponentBeginOverlap`
  (params (OverlappedComponent :type "PrimitiveComponent Object Reference") (OtherActor :type "Actor Object Reference") (OtherComp :type "PrimitiveComponent Object Reference") (OtherBodyIndex :type Integer) (bFromSweep :type Boolean) (SweepResult :type "HitResult Structure (by ref)"))
  ;[1 1 1] Overlaps
  (if (`KismetStringLibrary.EqualEqual_StrStr` (`KismetSystemLibrary.GetDisplayName` OtherActor) "WOLF")
    (set `self.is_overlapping` true)))

(event `self.Comida_bebida.OnComponentEndOverlap`
  (params (OverlappedComponent :type "PrimitiveComponent Object Reference") (OtherActor :type "Actor Object Reference") (OtherComp :type "PrimitiveComponent Object Reference") (OtherBodyIndex :type Integer))
  ;[1 1 1] Overlaps
  (if (`KismetStringLibrary.EqualEqual_StrStr` (`KismetSystemLibrary.GetDisplayName` OtherActor) "WOLF")
    (set `self.is_overlapping` false)))

(event `self.ReceiveTick`
  (params (DeltaSeconds :type "Float (single-precision)"))
  (bind _wolf (`self.WOLF`))
  (bind _wolf_2 (`self.WOLF`))
  ;[1 1 1] Comprobacion
  (if (and (`self.is_overlapping`) (`self.is_pressed`))
    (if (`self.Is_Comida`)
      (set `/Game/_HomelessDog/Blueprints/WOLF.Hambre` (+ (`/Game/_HomelessDog/Blueprints/WOLF.Hambre` _wolf_2) 20.0) _wolf_2)
      (else
        (set `/Game/_HomelessDog/Blueprints/WOLF.Sed` (+ (`/Game/_HomelessDog/Blueprints/WOLF.Sed` _wolf) 20.0) _wolf)))
    (`self.K2_DestroyActor`)))

(fn `UserConstructionScript`)